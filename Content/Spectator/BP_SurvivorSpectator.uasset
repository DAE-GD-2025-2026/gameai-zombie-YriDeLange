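; BP_SurvivorSpectator is a spectator camera that follows the survivor in the level.
; On BeginPlay it finds BP_Survivor, attaches itself with a location snap and relative rotation, and caches its player controller.
; IA_Zoom adjusts the clamped spring arm length in perspective mode, or the unclamped ortho width otherwise.
; A helper returns line trace start and end points along the camera's forward vector.
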(event Input|EnhancedActionEvents|EnhancedInputActionIA_Zoom
  (params (ActionValue :type Float%20%28double-precision%29) (ElapsedSeconds :type Float%20%28double-precision%29) (TriggeredSeconds :type Float%20%28double-precision%29) (InputAction :type Input%20Action%20Object%20Reference :default "/Game/Input/IA_Zoom.IA_Zoom"))
  (bind _camera (Variables|Default|GetCamera))
  (bind _zoomspeed (Variables|Default|GetZoomSpeed))
  (bind _returnvalue (* ActionValue _zoomspeed))
  (if (Utilities|Enum|Equal(Enum) (Variables|/Script/Engine.CameraComponent|GetProjectionMode (Variables|Default|GetCamera)) "Perspective")
    (Variables|/Script/Engine.SpringArmComponent|SetTargetArmLength (Variables|Default|GetSpringArm) (Math|Float|Clamp(Float) (+ _returnvalue (Variables|/Script/Engine.SpringArmComponent|GetTargetArmLength (Variables|Default|GetSpringArm))) (Variables|Default|GetMinZoom) (Variables|Default|GetMaxZoom)))
    (else
      (Class|CameraComponent|SetOrthoWidth _camera (+ _returnvalue (Variables|/Script/Engine.CameraComponent|GetOrthoWidth _camera))))))

(event EventBeginPlay
  (bind _returnvalue (Actor|GetActorOfClass "/Game/Suvivor/BP_Survivor.BP_Survivor_C"))
  (bind _output_get (Variables|Default|SetSurvivor _returnvalue))
  (Transformation|AttachActorToActor _output_get "None" "SnapToTarget" "KeepRelative" "KeepRelative" true)
  (bind _asplayer_controller (Utilities|Casting|CastToPlayerController (Pawn|GetController)))
  (Variables|Default|SetPlayerController _asplayer_controller))

(fn ConstructionScript)

(fn GetTargetLineTraceStartEnd
  (bind _camera (Variables|Default|GetCamera))
  (bind _returnvalue (Transformation|GetWorldLocation _camera))
  (return _returnvalue (+ _returnvalue (* (Math|Vector|GetForwardVector _camera) (LocalVariables|GetTraceDistance)))))